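; BP_Fire is a fire hazard or effect actor that reacts when the VR pawn overlaps its box.
; On overlap it spawns emitters at both motion controller aim locations, with scaled-down smoke on the left and no template set on the right.
; It attaches its own ParticleSystem1, not the spawned emitters, to the right aim and then the left, so that component ends up on the left.
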(event OnComponentBeginOverlap(Box)
  (params (OverlappedComponent :type Primitive%20Component%20Object%20Reference) (OtherActor :type Actor%20Object%20Reference) (OtherComp :type Primitive%20Component%20Object%20Reference) (OtherBodyIndex :type Integer) (bFromSweep :type Boolean) (SweepResult :type Hit%20Result%20Structure%20%28by%20ref%29))
  (bind _asvrpawn (Utilities|Casting|CastToVRPawn OtherActor))
  (Effects|SpawnEmitteratLocation 0 (Transformation|GetWorldLocation (Variables|/Game/VRTemplate/Blueprints/VRPawn.VRPawn_C|GetMotionControllerRightAim _asvrpawn)))
  (Transformation|AttachComponentToComponent (Variables|Default|GetParticleSystem1) (Variables|/Game/VRTemplate/Blueprints/VRPawn.VRPawn_C|GetMotionControllerRightAim _asvrpawn) "None" "KeepRelative" "KeepRelative" "KeepRelative" true)
  (Effects|SpawnEmitteratLocation "/Game/StarterContent/Particles/P_Smoke.P_Smoke" (Transformation|GetWorldLocation (Variables|/Game/VRTemplate/Blueprints/VRPawn.VRPawn_C|GetMotionControllerLeftAim _asvrpawn)) "0, 0, 0" "0.070000,0.070000,0.070000")
  (Transformation|AttachComponentToComponent (Variables|Default|GetParticleSystem1) (Variables|/Game/VRTemplate/Blueprints/VRPawn.VRPawn_C|GetMotionControllerLeftAim _asvrpawn) "None" "KeepRelative" "KeepRelative" "KeepRelative" true))

(fn ConstructionScript)